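; Shooting-mode HUD that creates and displays the HUD widget and sets game-only input with the cursor hidden on BeginPlay.
; It binds to the local BP_ShootingPlayerState's health, magazine and SH dispatchers, retrying by timer until the cast succeeds, and pushes initial values to the widget.
; BindPlayerState hooks any given player's name and kill/death dispatchers to refresh the user list.
; The name-refresh retry timer targets UpdateUserPlayerState, which this Blueprint does not define.
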(event `self.ReceiveBeginPlay`
  (bind _returnvalue (`GameplayStatics.GetPlayerController` 0))
  (`KismetSystemLibrary.PrintString` "ShootingHud BeginPlay" true true (struct :`G` 1.0 :`A` 1.0) 60.0)
  (bind _returnvalue_2 (`|CreateWidget` "/Game/Shooting/Widget/ShootingHudWidget.ShootingHudWidget_C"))
  (bind _output_get (set `self.HudWidget` _returnvalue_2))
  (`UserWidget.AddToViewport` _output_get 0)
  (`self.BindMyPlayerState`)
  (`WidgetBlueprintLibrary.SetInputMode_GameOnly` _returnvalue)
  (set `PlayerController.bShowMouseCursor` false _returnvalue))

(fn `BindMyPlayerState`
  (bind _asbp_shooting_player_state (cast `/Game/Shooting/GameMode/BP_ShootingPlayerState` (`Controller.PlayerState` (`GameplayStatics.GetPlayerController` 0)))
    (:`then`
      (`|ExecutionSequence`
        (:`then_0`
          ;[1 1 1] Hp Update
          (add `/Game/Shooting/GameMode/BP_ShootingPlayerState.EventDispatcher_UpdateHp` _asbp_shooting_player_state (`|CreateDelegate` :!event `EventMyUpdateHp`))
          ;[1 1 1] 로딩 후 Default 값 전달
          ; 게임 시작 직후 피 100
          (`self.EventMyUpdateHp` (`/Game/Shooting/GameMode/BP_ShootingPlayerState.CurHp` _asbp_shooting_player_state) (`/Game/Shooting/GameMode/BP_ShootingPlayerState.MaxHp` _asbp_shooting_player_state))
          (`self.EventMyMag` (`/Game/Shooting/GameMode/BP_ShootingPlayerState.Mag` _asbp_shooting_player_state))
          ;[1 1 1] Mag Update
          (add `/Game/Shooting/GameMode/BP_ShootingPlayerState.EventDispatcher_UpdateMag` _asbp_shooting_player_state (`|CreateDelegate` :!event `EventMyMag`)))
        (:`then_1`
          (add `/Game/Shooting/GameMode/BP_ShootingPlayerState.EventDispatcher_UpdateSH` _asbp_shooting_player_state (`|CreateDelegate` :!event `EventMyUpdateSH`))
          (`self.EventMyUpdateSH` (`/Game/Shooting/GameMode/BP_ShootingPlayerState.CurSH` _asbp_shooting_player_state) (`/Game/Shooting/GameMode/BP_ShootingPlayerState.MaxSH` _asbp_shooting_player_state)))))
    (:`CastFailed`
      (`KismetSystemLibrary.K2_SetTimer` null "BindMyPlayerState" 0.01))))

(fn `BindPlayerState`
  (params (PlayerState :type "/Game/Shooting/GameMode/BP_ShootingPlayerState Object Reference"))
  (`/Engine/EditorBlueprintResources/StandardMacros.IsValid` PlayerState
    (:`Is Valid`
      (add `/Game/Shooting/GameMode/BP_ShootingPlayerState.EventDispatcher_ScoreUserName` PlayerState (`|CreateDelegate` :!event `EventUserName`))
      (`self.EventUserName` (`/Game/Shooting/GameMode/BP_ShootingPlayerState.UserName` PlayerState))
      (add `/Game/Shooting/GameMode/BP_ShootingPlayerState.EventDispatcher_UpdateKillDeath` PlayerState (`|CreateDelegate` :!event `EventUserKillDeath`)))))

(fn `EventMyMag`
  (params (Mag :type Integer))
  (`/Game/Shooting/Widget/ShootingHudWidget.UpdateMag` (`self.HudWidget`) Mag))

(fn `EventMyUpdateAmmo`
  (params (CurAmmo :type Integer))
  (`/Game/Shooting/Widget/ShootingHudWidget.UpdateAmmo` (`self.HudWidget`) CurAmmo))

(fn `EventMyUpdateHp`
  (params (CurHp :type "Float (double-precision)") (MaxHp :type "Float (double-precision)"))
  (`/Game/Shooting/Widget/ShootingHudWidget.UpdateHp` (`self.HudWidget`) CurHp MaxHp))

(fn `EventMyUpdateSH`
  (params (CurSH :type "Float (double-precision)") (MaxSH :type "Float (double-precision)"))
  (`/Game/Shooting/Widget/ShootingHudWidget.UpdateSH` (`self.HudWidget`) CurSH MaxSH))

(fn `EventUserKillDeath`
  (params (Kill :type Integer) (Death :type Integer))
  (`self.UpdateUserKillDeath`))

(fn `EventUserName`
  (params (UserName :type String))
  (`self.UpdateUserState`))

(fn `UpdateUserKillDeath`
  (bind _hudwidget (`self.HudWidget`)
    (:`then`
      (`/Game/Shooting/Widget/ShootingHudWidget.UpdateUserList` _hudwidget))
    (:`else`
      (`KismetSystemLibrary.K2_SetTimer` null "UpdateUserKillDeath" 0.01))))

(fn `UpdateUserState`
  (bind _hudwidget (`self.HudWidget`)
    (:`then`
      (`/Game/Shooting/Widget/ShootingHudWidget.UpdateUserList` _hudwidget))
    (:`else`
      (`KismetSystemLibrary.K2_SetTimer` null "UpdateUserPlayerState" 0.01))))

(fn `UserConstructionScript`)