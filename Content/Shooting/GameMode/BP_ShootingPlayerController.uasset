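; Player controller for the shooting game mode that passes the local player's user name to their player state.
; On possession the server calls a client event, which reads UserName from BP_ShootingGameInst.
; The client sends it back through a server event that sets it on BP_ShootingPlayerState.
; Each step has a debug PrintString with screen and log output turned off.
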(event `self.ReceivePossess`
  (params (PossessedPawn :type "Pawn Object Reference"))
  ;[1 0 0] Server
  (`KismetSystemLibrary.PrintString` (`KismetStringLibrary.Concat_StrStr` "ShootingPC OnPossess -" (`KismetSystemLibrary.GetDisplayName` PossessedPawn)) false false (struct :`G` 0.66 :`B` 1.0 :`A` 1.0) 60.0)
  (`self.ResOnPossess` PossessedPawn))

(event `ResOnPossess`
  (params (PossessedPawn :type "Pawn Object Reference"))
  ;[1 1 1] Client
  (`KismetSystemLibrary.PrintString` (`KismetStringLibrary.Concat_StrStr` "ShootingPC ResOnPossess Pawn -" (`KismetSystemLibrary.GetDisplayName` PossessedPawn)) false false (struct :`G` 0.66 :`B` 1.0 :`A` 1.0) 60.0)
  (bind _asbp_shooting_game_inst (cast `/Game/Shooting/GameMode/BP_ShootingGameInst` (`GameplayStatics.GetGameInstance`)))
  (`self.ReqNewUserName` (`/Game/Shooting/GameMode/BP_ShootingGameInst.UserName` _asbp_shooting_game_inst)))

(event `ReqNewUserName`
  (params (UserName :type String))
  ;[1 0 0] Server
  (`KismetSystemLibrary.PrintString` (`KismetStringLibrary.Concat_StrStr` "ShootingPC ReqNewUserName -" UserName) false false (struct :`G` 0.66 :`B` 1.0 :`A` 1.0) 60.0)
  (bind _asbp_shooting_player_state (cast `/Game/Shooting/GameMode/BP_ShootingPlayerState` (`self.PlayerState`)))
  (`/Game/Shooting/GameMode/BP_ShootingPlayerState.SetUserName` _asbp_shooting_player_state UserName))

(fn `UserConstructionScript`)