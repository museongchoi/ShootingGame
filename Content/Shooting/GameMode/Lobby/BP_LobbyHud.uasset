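; Lobby HUD that creates and shows the lobby widget, switching input to UI only with a visible mouse cursor.
; It binds to the local BP_LobbyPlayerState's lobby-state dispatcher to update the player's own state in the widget.
; BindPlayerState hooks a given player state's name and lobby-state dispatchers, with handlers that refresh the user list.
; Short timers retry by function name until the local player state or widget is ready.
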(event `self.ReceiveBeginPlay`
  (bind _returnvalue (`GameplayStatics.GetPlayerController` 0))
  (bind _returnvalue_2 (`|CreateWidget` "/Game/Shooting/Widget/Lobby/LobbyHudWidget.LobbyHudWidget_C"))
  (bind _output_get (set `self.HudWidget` _returnvalue_2))
  (`UserWidget.AddToViewport` _output_get 0)
  (`WidgetBlueprintLibrary.SetInputMode_UIOnlyEx` _returnvalue null)
  (set `PlayerController.bShowMouseCursor` true _returnvalue)
  (`self.BindMyPlayerState`))

(fn `BindMyPlayerState`
  (bind _asbp_lobby_player_state (cast `/Game/Shooting/GameMode/Lobby/BP_LobbyPlayerState` (`Controller.PlayerState` (`GameplayStatics.GetPlayerController` 0)))
    (:`then`
      (add `/Game/Shooting/GameMode/Lobby/BP_LobbyPlayerState.EventDispatcher_LobbyState` _asbp_lobby_player_state (`|CreateDelegate` :!event `EventMyLobbyState`))
      (`self.EventMyLobbyState` (`/Game/Shooting/GameMode/Lobby/BP_LobbyPlayerState.LobbyState` _asbp_lobby_player_state)))
    (:`CastFailed`
      (`KismetSystemLibrary.K2_SetTimer` null "BindMyPlayerState" 0.01))))

(fn `BindPlayerState`
  (params (PlayerState :type "/Game/Shooting/GameMode/Lobby/BP_LobbyPlayerState Object Reference"))
  (`/Engine/EditorBlueprintResources/StandardMacros.IsValid` PlayerState
    (:`Is Valid`
      (add `/Game/Shooting/GameMode/Lobby/BP_LobbyPlayerState.EventDispatcher_UserName` PlayerState (`|CreateDelegate` :!event `EventUserName`))
      (`self.EventUserName` (`/Game/Shooting/GameMode/Lobby/BP_LobbyPlayerState.UserName` PlayerState))
      (add `/Game/Shooting/GameMode/Lobby/BP_LobbyPlayerState.EventDispatcher_LobbyState` PlayerState (`|CreateDelegate` :!event `Update Lobby State`)))))

(fn `EventMyLobbyState`
  (params (LobbyState :type "/Game/Shooting/Data/EN_LobbyPlayerState Enum" :default "NewEnumerator0"))
  (`/Game/Shooting/Widget/Lobby/LobbyHudWidget.ChangeMyLobbyState` (`self.HudWidget`) LobbyState))

(fn `EventUserName`
  (params (UserName :type String))
  (`self.UpdatePlayerState`))

(fn `Update Lobby State`
  (params (LobbyState :type "/Game/Shooting/Data/EN_LobbyPlayerState Enum" :default "NewEnumerator0"))
  (bind _hudwidget (`self.HudWidget`)
    (:`then`
      (`/Game/Shooting/Widget/Lobby/LobbyHudWidget.Update User List` _hudwidget))
    (:`else`
      (`KismetSystemLibrary.K2_SetTimer` null "Update Lobby State" 0.01))))

(fn `UpdatePlayerState`
  (bind _hudwidget (`self.HudWidget`)
    (:`then`
      (`/Game/Shooting/Widget/Lobby/LobbyHudWidget.Update User List` _hudwidget))
    (:`else`
      (`KismetSystemLibrary.K2_SetTimer` null "UpdatePlayerState" 0.01))))

(fn `UserConstructionScript`)