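; Lobby game state that starts a five-second countdown once all players are ready and then moves the session into the match map.
; UpdateGameState, on authority, checks every lobby player state and switches between waiting and countdown, resetting the timer.
; Tick advances the countdown and, on expiry, sets the final state and server-travels everyone to InGameMap.
; The replicated state's OnRep prints a debug string and fires an event dispatcher.
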(event `self.ReceiveTick`
  (params (DeltaSeconds :type "Float (single-precision)"))
  (if (`|EnumEquality` (`self.GameState`) "NewEnumerator1")
    (bind _output_get (set `self.CountDownDS` (+ DeltaSeconds (`self.CountDownDS`))))
    (if (> _output_get 5.0)
      (set `self.CountDownDS` 5.0)
      (set `self.GameState` "NewEnumerator2")
      (`self.DoMoveLevel`))))

(fn `CheckAllComplete`
  (returns (IsAllComplete :type Boolean))
  (bind _outactors (`GameplayStatics.GetAllActorsOfClass` "/Game/Shooting/GameMode/Lobby/BP_LobbyPlayerState.BP_LobbyPlayerState_C"))
  (for _array_element _outactors
    (if (`|EnumInequality` (`/Game/Shooting/GameMode/Lobby/BP_LobbyPlayerState.LobbyState` _array_element) "NewEnumerator1")
      (return false)))
  (return true))

(fn `DoMoveLevel`
  ;[1 1 1] 세션에 같이 있는 플레이어들과 같이 이동
  (`KismetSystemLibrary.ExecuteConsoleCommand` "servertravel  InGameMap" null))

(fn `OnRep_GameState`
  (`KismetSystemLibrary.PrintString` (`KismetStringLibrary.Concat_StrStr` "OnRep_GameState - " (`|GetEnumeratorNameAsString` (`self.GameState`))) true true (struct :`G` 0.66 :`B` 1.0 :`A` 1.0) 60.0)
  (`self.EventDispatcher_GameState` (`self.GameState`)))

(fn `UpdateGameState`
  (`/Engine/EditorBlueprintResources/ActorMacros.Switch Has Authority`
    (:`Authority`
      (if (`|EnumInequality` (`self.GameState`) "NewEnumerator2")
        (if (`self.CheckAllComplete`)
          (set `self.CountDownDS` 0.0)
          (set `self.GameState` "NewEnumerator1")
          (else
            (set `self.CountDownDS` 0.0)
            (set `self.GameState` "NewEnumerator0")))))))

(fn `UserConstructionScript`)