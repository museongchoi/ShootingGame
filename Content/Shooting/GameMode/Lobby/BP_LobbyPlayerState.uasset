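; BP_LobbyPlayerState holds each player's name and Ready/Complete lobby state for the lobby.
; On BeginPlay it binds itself to the local player controller's BP_LobbyHud.
; RepNotify functions on both values print debug text and fire event dispatchers to announce changes.
; ChangeLobbyState, commented as server-executed via the lobby controller, toggles the state and then tells BP_LobbyGameState to update.
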(event `self.ReceiveBeginPlay`
  (`KismetSystemLibrary.PrintString` "PlayerStateBeginPlay" true true (struct :`G` 0.66 :`B` 1.0 :`A` 1.0) 60.0)
  (bind _asbp_lobby_hud (cast `/Game/Shooting/GameMode/Lobby/BP_LobbyHud` (`PlayerController.GetHUD` (`GameplayStatics.GetPlayerController` 0))))
  (`/Game/Shooting/GameMode/Lobby/BP_LobbyHud.BindPlayerState` _asbp_lobby_hud self))

(fn `ChangeLobbyState`
  ;[1 0.005208 0.005208] Server : LobbyController 의 해당 함수 실행 부분이 서버에서 실행되기 때문에 해당 함수는 Server 에서 실행하는 것이다
  (`|ExecutionSequence`
    (:`then_0`
      (switch `/Game/Shooting/Data/EN_LobbyPlayerState` (`self.LobbyState`)
        (:`NewEnumerator0`
          (set `self.LobbyState` "NewEnumerator1"))
        (:`NewEnumerator1`
          (set `self.LobbyState` "NewEnumerator0"))))
    (:`then_1`
      (bind _asbp_lobby_game_state (cast `/Game/Shooting/GameMode/Lobby/BP_LobbyGameState` (`GameplayStatics.GetGameState`)))
      (`/Game/Shooting/GameMode/Lobby/BP_LobbyGameState.UpdateGameState` _asbp_lobby_game_state))))

(fn `OnRep_LobbyState`
  ;[1 1 1] Client
  (`KismetSystemLibrary.PrintString` (`KismetStringLibrary.Concat_StrStr` "LobbyState - " (`|GetEnumeratorNameAsString` (`self.LobbyState`))))
  (`self.EventDispatcher_LobbyState` (`self.LobbyState`)))

(fn `OnRep_UserName`
  ;[1 1 1] Client : Server 에서 변경점이 있을시 실행되는 부분
  (`KismetSystemLibrary.PrintString` (`KismetStringLibrary.Concat_StrStr` "BP_LobbyPlayerState OnRepUserName -" (`self.UserName`)) true true (struct :`G` 0.66 :`B` 1.0 :`A` 1.0) 60.0)
  (`self.EventDispatcher_UserName` (`self.UserName`)))

(fn `SetUserName`
  (params (UserName :type String))
  (set `self.UserName` UserName))

(fn `UserConstructionScript`)