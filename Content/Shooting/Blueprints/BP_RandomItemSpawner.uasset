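; Item spawner actor that places a random class from its Items list at its own transform and periodically replaces it.
; A randomized timer runs SpawnItem, which on authority only deletes the current item, creates a new one and re-arms the timer with a fresh random delay.
; An OnDestroyed binding reschedules a fixed-delay respawn when the item disappears, and is unbound before the spawner's own deletions.
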(event `self.ReceiveBeginPlay`
  (`KismetSystemLibrary.K2_SetTimer` null "SpawnItem" (`KismetMathLibrary.RandomFloatInRange` 5.0 10.0)))

(fn `CreateItem`
  (bind _items (`self.Items`))
  (if (`KismetArrayLibrary.Array_IsNotEmpty` _items)
    (bind _returnvalue (`|SpawnActorFromClass` (`KismetArrayLibrary.Array_Random` _items) (`self.GetTransform`) "Undefined" "MultiplyWithRoot" null null))
    (bind _output_get (set `self.SpawnedItem` _returnvalue))
    (if (`self.IsActorBeingDestroyed` _output_get)
      (`self.EventItemDestroy` null)
      (else
        (add `self.OnDestroyed` _output_get (`|CreateDelegate` :!event `EventItemDestroy`))))))

(fn `DeleteItem`
  (bind _spawneditem (`self.SpawnedItem`)
    (:`then`
      (remove `self.OnDestroyed` _spawneditem (`|CreateDelegate` :!event `EventItemDestroy`))
      (`self.K2_DestroyActor` _spawneditem))
    (:`else`)))

(fn `EventItemDestroy`
  (params (DestroyedActor :type "Actor Object Reference"))
  (`|ExecutionSequence`
    (:`then_0`
      (if (`KismetSystemLibrary.K2_TimerExists` null "SpawnItem")
        (`KismetSystemLibrary.K2_ClearTimer` null "SpawnItem")))
    (:`then_1`
      (`KismetSystemLibrary.K2_SetTimer` null "SpawnItem" 5.0))))

(fn `SpawnItem`
  (`/Engine/EditorBlueprintResources/ActorMacros.Switch Has Authority`
    (:`Authority`
      (`self.DeleteItem`)
      (`self.CreateItem`)
      (`|ExecutionSequence`
        (:`then_0`
          (if (`KismetSystemLibrary.K2_TimerExists` null "SpawnItem")
            (`KismetSystemLibrary.K2_ClearTimer` null "SpawnItem")))
        (:`then_1`
          (`KismetSystemLibrary.K2_SetTimer` null "SpawnItem" (`KismetMathLibrary.RandomFloatInRange` 5.0 10.0) true))))))

(fn `UserConstructionScript`)