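; Machine gun weapon Blueprint that provides automatic fire while the trigger is held.
; EventTigger shoots immediately on press and starts a looping DoShoot timer paced by GetShootDelayByRPM, then clears it on release.
; Each DoShoot checks IsCanShoot and a valid Character, then plays the WeaponData fire montage, or stops the timer if either check fails.
; DoShoot itself spawns no projectile or trace, only the montage.
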(fn `DoShoot`
  (bind _iscanshoot (`/Game/Shooting/Blueprints/BPI_Weapon.IsCanShoot`))
  (if _iscanshoot
    (bind _character (`self.Character`)
      (:`then`
        (`Character.PlayAnimMontage` _character (`.FireMontage_22_7F459E2645BB63EF568032BA9BA027B0` (break `/Game/Shooting/Data/ST_WeaponData` (`self.WeaponData`))) 1.0 "None"))
      (:`else`
        (`KismetSystemLibrary.K2_ClearTimer` null "DoShoot" :!label _label)))
    (else
      (goto _label))))

(fn `EventTigger`
  (params (IsPressed :type Boolean))
  (returns (bResult :type Boolean))
  (if IsPressed
    (`self.DoShoot`)
    (`KismetSystemLibrary.K2_SetTimer` null "DoShoot" (`self.GetShootDelayByRPM`) true)
    (else
      (`KismetSystemLibrary.K2_ClearTimer` null "DoShoot")))
  (return false))

(fn `UserConstructionScript`
  (`parent.UserConstructionScript`))