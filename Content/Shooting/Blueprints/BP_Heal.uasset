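; BP_Heal is a health pickup for the shooting game that restores HP to a character overlapping its sphere.
; On overlap, only the server checks the actor through IsCanHealActor, which requires a BP_ShootingCharacter with a living BP_ShootingPlayerState below max HP.
; If eligible, it calls AddHeal on that player state with a fixed amount and destroys itself, so ineligible overlaps leave the pickup in place.
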(event `self.Sphere.OnComponentBeginOverlap`
  (params (OverlappedComponent :type "PrimitiveComponent Object Reference") (OtherActor :type "Actor Object Reference") (OtherComp :type "PrimitiveComponent Object Reference") (OtherBodyIndex :type Integer) (bFromSweep :type Boolean) (SweepResult :type "HitResult Structure (by ref)"))
  (`/Engine/EditorBlueprintResources/ActorMacros.Switch Has Authority`
    (:`Authority`
      (bind (_iscanheal _player_state) (`self.IsCanHealActor` OtherActor))
      (if _iscanheal
        (`/Game/Shooting/GameMode/BP_ShootingPlayerState.AddHeal` _player_state 100.0)
        (`self.K2_DestroyActor`)))))

(fn `IsCanHealActor`
  (params (Actor :type "Actor Object Reference"))
  (returns (IsCanHeal :type Boolean) (`Player State` :type "/Game/Shooting/GameMode/BP_ShootingPlayerState Object Reference"))
  (bind _asbp_shooting_character (cast `/Game/Shooting/GameMode/BP_ShootingCharacter` Actor)
    (:`then`
      (bind _asbp_shooting_player_state (cast `/Game/Shooting/GameMode/BP_ShootingPlayerState` (`Pawn.PlayerState` _asbp_shooting_character))
        (:`then`
          (if (not (`/Game/Shooting/GameMode/BP_ShootingPlayerState.IsDeath` _asbp_shooting_player_state))
            (return (< (`/Game/Shooting/GameMode/BP_ShootingPlayerState.CurHp` _asbp_shooting_player_state) (`/Game/Shooting/GameMode/BP_ShootingPlayerState.MaxHp` _asbp_shooting_player_state)) _asbp_shooting_player_state)))
        (:`CastFailed`
          (return false null))))
    (:`CastFailed`
      (return false null))))

(fn `UserConstructionScript`)