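; Burst fire mode for a shooting weapon, playing a three-round burst per trigger press.
; EventTigger ignores releases and presses during an active burst, otherwise it resets the counter, fires at once and starts a looping RPM-based timer.
; Each DoShoot call plays the WeaponData fire montage on the Character and counts it, clearing the timer after the third or when shooting is disallowed or the Character is invalid.
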(fn `DoShoot`
  (bind _iscanshoot (`/Game/Shooting/Blueprints/BPI_Weapon.IsCanShoot`))
  (if _iscanshoot
    (bind _character (`self.Character`)
      (:`then`
        (`Character.PlayAnimMontage` _character (`.FireMontage_22_7F459E2645BB63EF568032BA9BA027B0` (break `/Game/Shooting/Data/ST_WeaponData` (`self.WeaponData`))) 1.0 "None")
        (bind _result (`/Engine/EditorBlueprintResources/StandardMacros.IncrementFloat` (`self.BustCnt`))
          (:`  `
            (if (>= _result 3.0)
              (set `self.BustCnt` 0.0)
              (`KismetSystemLibrary.K2_ClearTimer` null "DoShoot")))))
      (:`else`
        (`KismetSystemLibrary.K2_ClearTimer` null "DoShoot" :!label _label)))
    (else
      (goto _label))))

(fn `EventTigger`
  (params (IsPressed :type Boolean))
  (returns (bResult :type Boolean))
  (if IsPressed
    (if (not (`KismetSystemLibrary.K2_TimerExists` null "DoShoot"))
      (set `self.BustCnt` 0.0)
      (`self.DoShoot`)
      (`KismetSystemLibrary.K2_SetTimer` null "DoShoot" (`self.GetShootDelayByRPM`) true)
      (return false))))

(fn `UserConstructionScript`
  (`parent.UserConstructionScript`))